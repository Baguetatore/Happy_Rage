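; BP_Transpalette is a pallet jack enemy Character that reacts when the player is Enragé (frustrated).
; Pawn sensing drives a tick-delayed loop that turns it toward the player, then, once Boom reaches 1, alternates aiming and launched charges.
; Damage drains its health toward TranspalDead and lowers player Frustration, while capsule overlap calls SeFrustrerCalmer on an enraged player.
; PuzzleLaunch separately launches it forward.
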(event OnSeePawn(PawnSensing)
  (params (Pawn :type Pawn%20Object%20Reference))
  (bind _returnvalue (Transformation|GetActorRotation))
  (bind _returnvalue_2 (Math|Vector|GetForwardVector _returnvalue))
  (bind _returnvalue_3 (* _returnvalue_2 8e+03))
  ;[0.15 0.15 0.15 0.5] Phase 1 de la Transpalette où elle se pivote vers le joueur lorsque le joueur est frustré
  (bind _asbp_third_person_character (Utilities|Casting|CastToBP_ThirdPersonCharacter Pawn))
  (if (and (Variables|/Game/MyContent/BP_ThirdPersonCharacter.BP_ThirdPersonCharacter_C|GetEnragé _asbp_third_person_character) (not (Variables|Default|GetPhase2))) :!label _label
    (Variables|Default|SetLaunch? false)
    (Transformation|SetActorRotation (Math|Rotator|FindLookatRotation (Transformation|GetActorLocation) (Transformation|GetActorLocation _asbp_third_person_character)))
    (else
      (Variables|Default|SetLaunch? true)))
  (Utilities|FlowControl|DelayUntilNextTick)
  ;[0.15 0.15 0.15 0.5] Phase 2 lorsque la transpalette détruit les deux murs (BP_Fissure) où il pivote vers le joueur, attend quelques secondes avant de charger
  (if (and (Variables|/Game/MyContent/BP_ThirdPersonCharacter.BP_ThirdPersonCharacter_C|GetEnragé _asbp_third_person_character) (>= (Variables|Default|GetBoom) 1)) :!label _label_2
    (if (Variables|Default|GetLooking)
      (Variables|Default|SetPhase2 true)
      (Transformation|SetActorRotation (Math|Rotator|FindLookatRotation (Transformation|GetActorLocation) (Transformation|GetActorLocation _asbp_third_person_character)))
      (Utilities|FlowControl|Delay 5.0)
      (Variables|Default|SetLooking false)
      (goto _label_2)
      (else
        (Variables|Default|SetPhase2 true)
        (Utilities|FlowControl|Delay 2.0)
        (Variables|Default|SetImpacteRhino true)
        (Character|LaunchCharacter (Math|Vector|MakeVector (.x _returnvalue_3) (.y _returnvalue_3) 0.0) false false)
        (Variables|Default|SetLooking true)
        (Utilities|FlowControl|Delay 3.0)
        (goto _label_2)))
    (else
      (Utilities|FlowControl|DelayUntilNextTick)
      (goto _label))))

(event OnComponentBeginOverlap(Capsule)
  (params (OverlappedComponent :type Primitive%20Component%20Object%20Reference) (OtherActor :type Actor%20Object%20Reference) (OtherComp :type Primitive%20Component%20Object%20Reference) (OtherBodyIndex :type Integer) (bFromSweep :type Boolean) (SweepResult :type Hit%20Result%20Structure%20%28by%20ref%29))
  ;[0.15 0.15 0.15 0.5] Fait des dégats lorsque le joueur est frustré et rentre en collision avec sa tête
  (bind _asbp_third_person_character (Utilities|Casting|CastToBP_ThirdPersonCharacter OtherActor :!label _label))
  (if (Variables|/Game/MyContent/BP_ThirdPersonCharacter.BP_ThirdPersonCharacter_C|GetEnragé _asbp_third_person_character)
    (Default|SeFrustrer/Calmer _asbp_third_person_character 80)
    (else
      (Utilities|FlowControl|DelayUntilNextTick)
      (goto _label))))

(event Custom|PuzzleLaunch
  (bind _returnvalue (Transformation|GetActorRotation))
  (bind _returnvalue_2 (Math|Vector|GetForwardVector _returnvalue))
  (bind _returnvalue_3 (* _returnvalue_2 1e+04))
  ;[0.15 0.15 0.15 0.5] Launch le character lorsque le joueur intéragit avec
  (Character|LaunchCharacter (Math|Vector|MakeVector (.x _returnvalue_3) (.y _returnvalue_3) 0.0) false false))

(event Game|Damage|EventAnyDamage
  (params (Damage :type Float%20%28single-precision%29) (DamageType :type Damage%20Type%20Object%20Reference) (InstigatedBy :type Controller%20Object%20Reference) (DamageCauser :type Actor%20Object%20Reference))
  ;[1 0.9343 0 0.5] Gestion des dégâts sur le mannequin
  ;;[1 0.00746 0 0.5] Baisse la frustration quand le mannequin prend des dégâts
  (bind _asbp_third_person_character (Utilities|Casting|CastToBP_ThirdPersonCharacter (Game|GetPlayerCharacter 0)))
  (Variables|/Game/MyContent/BP_ThirdPersonCharacter.BP_ThirdPersonCharacter_C|SetFrustration _asbp_third_person_character (- (Variables|/Game/MyContent/BP_ThirdPersonCharacter.BP_ThirdPersonCharacter_C|GetFrustration _asbp_third_person_character) Damage))
  ;;[1 0.8187 0 0.5] L'ennemi perd de la vie quand il prend des dégâts, il passe en mode ragdoll lorsque ses PV sont à 0
  (Variables|Default|SetHPTranspal (- (Variables|Default|GetHPTranspal) Damage))
  (if (<= (Variables|Default|GetHPTranspal) 0)
    (Variables|Default|SetTranspalDead true)))

(fn ConstructionScript)