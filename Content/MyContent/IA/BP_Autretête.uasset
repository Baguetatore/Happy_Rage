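; Enemy that watches a frustrated (IsZehef) player through PawnSensing and launches its Cone mesh as a projectile.
; After turning to the player and waiting, it flashes the cone's material as a one-time warning, then applies a forward physics impulse unless NOLAUNCH is set.
; Sphere overlap repeatedly raises SeFrustrerCalmer while CanDamage is true, or enables cone physics on a bat impact.
; A per-tick velocity check after hits is meant to disable damage on the ground.
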(event OnSeePawn(PawnSensing)
  (params (Pawn :type Pawn%20Object%20Reference))
  ;[0.15 0.15 0.15 0.5] Suit le joueur du regard s'il est frustré
  (bind _asbp_third_person_character (Utilities|Casting|CastToBP_ThirdPersonCharacter Pawn))
  (if (Variables|/Game/MyContent/BP_ThirdPersonCharacter.BP_ThirdPersonCharacter_C|GetIsZehef _asbp_third_person_character)
    (Transformation|SetActorRotation (Math|Rotator|FindLookatRotation (Transformation|GetActorLocation) (Transformation|GetActorLocation _asbp_third_person_character)))
    (Utilities|FlowControl|Delay 3.0)
    (Utilities|FlowControl|DoOnce false
      (:Completed
        (Variables|Default|SetFlashing true)
        (CallFunction|Flash)
        ;[0.9937 0 1 0.5] Comment
        (Utilities|FlowControl|Delay 2.0)
        (Variables|Default|SetFlashing false)
        (Rendering|Material|SetMaterial (Variables|Default|GetCone) 0 "/Game/StarterContent/Materials/M_Bleu.M_Bleu")
        (if (not (Variables|/Game/MyContent/BP_ThirdPersonCharacter.BP_ThirdPersonCharacter_C|GetNOLAUNCH _asbp_third_person_character))
          (Utilities|FlowControl|DoOnce false
            (:Completed
              (Variables|Default|SetcanDamage false)
              (Physics|SetSimulatePhysics (Variables|Default|GetCone) true)
              (Collision|SetCollisionEnabled (Variables|Default|GetCone) "PhysicsOnly")
              (Physics|AddImpulse (Variables|Default|GetCone) (* (Transformation|GetActorForwardVector) (Variables|Default|GetThrowforce)) "None" false)
              (Variables|Default|SetcanDamage true)
              (Utilities|FlowControl|Delay 3.0)
              (bind _asbp_mannequin_5 (Utilities|Casting|CastToBP_Mannequin5 Pawn))
              (Development|PrintString "Hello")
              (if (not (Variables|/Game/CHANGE/Trucquimarche/BP_Mannequin5.BP_Mannequin5_C|GetMORT _asbp_mannequin_5))
                (AI|AIMoveTo self (Variables|Default|GetPostion) 0 1e+05 false)))))))))

(event OnComponentBeginOverlap(Sphere)
  (params (OverlappedComponent :type Primitive%20Component%20Object%20Reference) (OtherActor :type Actor%20Object%20Reference) (OtherComp :type Primitive%20Component%20Object%20Reference) (OtherBodyIndex :type Integer) (bFromSweep :type Boolean) (SweepResult :type Hit%20Result%20Structure%20%28by%20ref%29))
  ;[0.15 0.15 0.15 0.5] Applique des dégats s'il ne rentre pas en contact avec la batte, si c'est le cas set physics
  (bind _asbp_third_person_character (Utilities|Casting|CastToBP_ThirdPersonCharacter OtherActor))
  (if (Variables|/Game/MyContent/BP_ThirdPersonCharacter.BP_ThirdPersonCharacter_C|GetImpacteBatte _asbp_third_person_character) :!label _label
    (Physics|SetSimulatePhysics (Variables|Default|GetCone) true)
    (Collision|SetCollisionEnabled (Variables|Default|GetCone) "PhysicsOnly")
    (elif (Variables|Default|GetcanDamage)
      (Default|SeFrustrer/Calmer _asbp_third_person_character 1)
      (Utilities|FlowControl|DelayUntilNextTick)
      (goto _label))))

(event OnComponentHit(Cone)
  (params (HitComponent :type Primitive%20Component%20Object%20Reference) (OtherActor :type Actor%20Object%20Reference) (OtherComp :type Primitive%20Component%20Object%20Reference) (NormalImpulse :type Vector :default "0, 0, 0") (Hit :type Hit%20Result%20Structure%20%28by%20ref%29))
  ;[0.15 0.15 0.15 0.5] Ne fait pas de dégat au sol
  (if (Class|KismetMathLibrary|EqualExactlyVectorVector (Transformation|GetVelocity) (Math|Conversions|ToVector(Float) (Math|Float|Floor (.Distance (Collision|BreakHitResult Hit))))) :!label _label
    (Variables|Default|SetcanDamage false)
    (else
      (Utilities|FlowControl|DelayUntilNextTick)
      (goto _label))))

(event Custom|Flash
  ;[0.02956 1 0.6105] Fait flasher l'objet
  ;;[0.9937 0 1 0.5] Comment
  (if (Variables|Default|GetFlashing) :!label _label
    (Rendering|Material|SetMaterial (Variables|Default|GetCone) 0 "/Engine/BasicShapes/BasicShapeMaterial.BasicShapeMaterial")
    (Utilities|FlowControl|Delay 0.2)
    (Rendering|Material|SetMaterial (Variables|Default|GetCone) 0 "/Game/StarterContent/Materials/M_Bleu.M_Bleu")
    (Utilities|FlowControl|Delay 0.2)
    (goto _label)))

(fn ConstructionScript)