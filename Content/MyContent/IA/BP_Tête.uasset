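; BP_Tête is a head hazard that throws itself at the player while PawnSensing sees them enraged (Enragé).
; Tick turns it toward the player, flashes its material, launches the Cone with a physics impulse, then eases it back toward its start unless struck.
; Sphere overlap pushes the head with physics on a bat impact, otherwise repeatedly calls SeFrustrerCalmer on the player while CanDamage is set.
; Sequencing relies on Delays and next-tick loops.
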(event OnSeePawn(PawnSensing)
  (params (Pawn :type Pawn%20Object%20Reference))
  ;[0.15 0.15 0.15 0.5] Suit le joueur du regard s'il est frustré
  (bind _asbp_third_person_character (Utilities|Casting|CastToBP_ThirdPersonCharacter Pawn :!label _label)
    (:then
      (if (Variables|/Game/MyContent/BP_ThirdPersonCharacter.BP_ThirdPersonCharacter_C|GetEnragé _asbp_third_person_character)
        (Variables|Default|SetLancer true)
        (Utilities|FlowControl|DelayUntilNextTick)
        (goto _label)
        (else
          (Variables|Default|SetLancer false))))
    (:CastFailed
      (Variables|Default|SetLancer false)
      (goto _label))))

(event OnComponentBeginOverlap(Sphere)
  (params (OverlappedComponent :type Primitive%20Component%20Object%20Reference) (OtherActor :type Actor%20Object%20Reference) (OtherComp :type Primitive%20Component%20Object%20Reference) (OtherBodyIndex :type Integer) (bFromSweep :type Boolean) (SweepResult :type Hit%20Result%20Structure%20%28by%20ref%29))
  (bind _returnvalue (Transformation|GetVelocity))
  (bind _returnvalue_2 (* _returnvalue 7e+02))
  ;[0.15 0.15 0.15 0.5] Applique des dégats s'il ne rentre pas en contact avec la batte, si c'est le cas set physics
  (bind _asbp_third_person_character (Utilities|Casting|CastToBP_ThirdPersonCharacter OtherActor))
  (if (Variables|/Game/MyContent/BP_ThirdPersonCharacter.BP_ThirdPersonCharacter_C|GetImpacteBatte _asbp_third_person_character) :!label _label
    (Physics|SetSimulatePhysics (Variables|Default|GetCone) true)
    (Collision|SetCollisionEnabled (Variables|Default|GetCone) "PhysicsOnly")
    (Development|PrintString "Hello")
    (Physics|AddForce (Variables|Default|GetCone) (Math|Vector|MakeVector (.x _returnvalue_2) (.y _returnvalue_2) (.z _returnvalue_2)) "None" false)
    (Variables|Default|SetTête%20frappée true)
    (Utilities|FlowControl|Delay 2.0)
    (Variables|Default|SetTête%20frappée false)
    (elif (Variables|Default|GetcanDamage)
      (Default|SeFrustrer/Calmer _asbp_third_person_character 100)
      (Utilities|FlowControl|DelayUntilNextTick)
      (goto _label))))

(event OnComponentHit(Cone)
  (params (HitComponent :type Primitive%20Component%20Object%20Reference) (OtherActor :type Actor%20Object%20Reference) (OtherComp :type Primitive%20Component%20Object%20Reference) (NormalImpulse :type Vector :default "0, 0, 0") (Hit :type Hit%20Result%20Structure%20%28by%20ref%29))
  ;[0.15 0.15 0.15 0.5] Ne fait pas de dégat au sol
  (if (Class|KismetMathLibrary|EqualExactlyVectorVector (Transformation|GetVelocity) (Math|Conversions|ToVector(Float) (Math|Float|Floor (.Distance (Collision|BreakHitResult Hit))))) :!label _label
    (Variables|Default|SetcanDamage false)
    (else
      (Utilities|FlowControl|DelayUntilNextTick)
      (goto _label))))

(event Custom|Flash
  ;[0.02956 1 0.6105] Fait flasher l'objet
  (if (Variables|Default|GetFlashing) :!label _label
    (Rendering|Material|SetMaterial (Variables|Default|GetCone) 0 "/Game/PROPS/MANNEQUIN_DISTANCE/tete_003.tete_003")
    (Utilities|FlowControl|Delay 0.2)
    (Rendering|Material|SetMaterial (Variables|Default|GetCone) 0 "/Game/StarterContent/Materials/M_Bleu.M_Bleu")
    (Utilities|FlowControl|Delay 0.2)
    (goto _label)))

(event EventBeginPlay
  (Variables|Default|SetPostion (Transformation|GetActorLocation)))

(event EventTick
  (params (DeltaSeconds :type Float%20%28single-precision%29))
  (bind _asbp_third_person_character (Utilities|Casting|CastToBP_ThirdPersonCharacter (Game|GetPlayerCharacter 0)))
  (if (Variables|Default|GetLancer)
    (Transformation|SetActorRotation (Math|Rotator|FindLookatRotation (Transformation|GetActorLocation) (Transformation|GetActorLocation _asbp_third_person_character)))
    (Utilities|FlowControl|Delay 3.0)
    ;[0.02956 1 0.6105] Fait flasher l'objet
    (Variables|Default|SetFlashing true)
    (CallFunction|Flash)
    (Utilities|FlowControl|Delay 2.0)
    (Variables|Default|SetFlashing false)
    (Rendering|Material|SetMaterial (Variables|Default|GetCone) 0 "/Game/StarterContent/Materials/M_Bleu.M_Bleu")
    (Variables|Default|SetcanDamage false)
    (if (Variables|Default|GetPositionInitiale)
      (Variables|Default|SetPositionInitiale false)
      (Physics|SetSimulatePhysics (Variables|Default|GetCone) true)
      (Collision|SetCollisionEnabled (Variables|Default|GetCone) "PhysicsOnly")
      (Utilities|FlowControl|Delay 0.1)
      (Physics|AddImpulse (Variables|Default|GetCone) (* (Transformation|GetActorForwardVector) (Variables|Default|GetThrowforce)) "None" false)
      (Utilities|FlowControl|Delay 5.0)
      (Variables|Default|SetPositionInitiale false)
      (Variables|Default|SetcanDamage true)
      (if (not (Variables|Default|GetTête%20frappée))
        (Utilities|FlowControl|Delay 2.5)
        (Physics|SetSimulatePhysics (Variables|Default|GetCone) false)
        (Collision|SetCollisionEnabled (Variables|Default|GetCone) "NoCollision")
        (if (not (Variables|Default|GetPositionInitiale))
          (Components|MoveComponentTo (Variables|Default|GetCone) (+ (Variables|Default|GetPostion) "0.000000,0.000000,-150.000000") "0, 0, 0" true false 5.0 false)
          (Utilities|FlowControl|Delay 5.0)
          (Variables|Default|SetPositionInitiale true))))))

(fn ConstructionScript)