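; BP_ManCrino1 is a mannequin enemy that takes damage and chases an enraged player.
; Any damage it receives lowers both the player character's Frustration and its own HPCrino, setting DeadBeat at zero health or below.
; PawnSensing triggers an AI MoveTo toward player 0 when it sees a third-person character whose Enragé flag is set.
; The ragdoll mentioned in the graph's comments is not implemented in this graph.
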(event OnSeePawn(PawnSensing)
  (params (Pawn :type Pawn%20Object%20Reference))
  ;[0.15 0.15 0.15 0.5] Suit le joueur
  (bind _asbp_third_person_character (Utilities|Casting|CastToBP_ThirdPersonCharacter Pawn))
  (if (Variables|/Game/MyContent/BP_ThirdPersonCharacter.BP_ThirdPersonCharacter_C|GetEnragé _asbp_third_person_character)
    (AI|AIMoveTo self "0, 0, 0" (Game|GetPlayerCharacter 0) 5.0 false)))

(event Game|Damage|EventAnyDamage
  (params (Damage :type Float%20%28single-precision%29) (DamageType :type Damage%20Type%20Object%20Reference) (InstigatedBy :type Controller%20Object%20Reference) (DamageCauser :type Actor%20Object%20Reference))
  ;[1 0.9343 0 0.5] Gestion des dégâts sur le mannequin
  ;;[1 0.00746 0 0.5] Baisse la frustration quand le mannequin prend des dégâts
  (bind _asbp_third_person_character (Utilities|Casting|CastToBP_ThirdPersonCharacter (Game|GetPlayerCharacter 0)))
  (Variables|/Game/MyContent/BP_ThirdPersonCharacter.BP_ThirdPersonCharacter_C|SetFrustration _asbp_third_person_character (- (Variables|/Game/MyContent/BP_ThirdPersonCharacter.BP_ThirdPersonCharacter_C|GetFrustration _asbp_third_person_character) Damage))
  ;;[1 0.8187 0 0.5] L'ennemi perd de la vie quand il prend des dégâts, il passe en mode ragdoll lorsque ses PV sont à 0
  (Variables|Default|SetHPCrino (- (Variables|Default|GetHPCrino) Damage))
  (if (<= (Variables|Default|GetHPCrino) 0)
    (Variables|Default|SetDeadBeat true)))

(fn ConstructionScript)