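; Test Blueprint for a Crino mannequin enemy whose rotating attack frustrates and launches the player.
; While the player is enraged, a polled FlipFlop alternates eased timeline spins with five-second pauses; AttackPlounge triggers a separate spin.
; Spins arm the DegatCrino overlap zone, which repeatedly calls SeFrustrerCalmer and launches the player along their forward vector.
; Damage taken lowers player Frustration and enemy HP, flagging DED at zero.
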(event OnComponentBeginOverlap(DegatCrino)
  (params (OverlappedComponent :type Primitive%20Component%20Object%20Reference) (OtherActor :type Actor%20Object%20Reference) (OtherComp :type Primitive%20Component%20Object%20Reference) (OtherBodyIndex :type Integer) (bFromSweep :type Boolean) (SweepResult :type Hit%20Result%20Structure%20%28by%20ref%29))
  ;[0.15 0.15 0.15 0.5] Damage en continu lorsque ça touche le joueur
  (bind _asbp_third_person_character (Utilities|Casting|CastToBP_ThirdPersonCharacter OtherActor))
  (Variables|Default|SetDegatOverlaped true)
  (if (and (Variables|Default|GetDegatCrinoHere?) (Variables|Default|GetDegatOverlaped)) :!label _label
    (Default|SeFrustrer/Calmer _asbp_third_person_character 20)
    (Character|LaunchCharacter _asbp_third_person_character (Math|Vector|MakeVector (.x (* (Math|Vector|GetForwardVector (Transformation|GetWorldRotation (Variables|/Script/Engine.Actor|GetRootComponent _asbp_third_person_character))) 5e+03)) (.y (* (Math|Vector|GetForwardVector (Transformation|GetWorldRotation (Variables|/Script/Engine.Actor|GetRootComponent _asbp_third_person_character))) 5e+03)) (+ (.z (* (Math|Vector|GetForwardVector (Transformation|GetWorldRotation (Variables|/Script/Engine.Actor|GetRootComponent _asbp_third_person_character))) 5e+03)) 1e+02)) false false))
  (Utilities|FlowControl|Delay 0.2)
  (goto _label))

(event OnComponentEndOverlap(DegatCrino)
  (params (OverlappedComponent :type Primitive%20Component%20Object%20Reference) (OtherActor :type Actor%20Object%20Reference) (OtherComp :type Primitive%20Component%20Object%20Reference) (OtherBodyIndex :type Integer))
  ;[0.15 0.15 0.15 0.5] Damage en continu lorsque ça touche le joueur
  (Utilities|Casting|CastToBP_ThirdPersonCharacter OtherActor)
  (Variables|Default|SetDegatOverlaped false))

(event OnComponentHit(DegatCrino)
  (params (HitComponent :type Primitive%20Component%20Object%20Reference) (OtherActor :type Actor%20Object%20Reference) (OtherComp :type Primitive%20Component%20Object%20Reference) (NormalImpulse :type Vector :default "0, 0, 0") (Hit :type Hit%20Result%20Structure%20%28by%20ref%29)))

(event Custom|AttackPlounge
  ;[0.15 0.15 0.15 0.5] Animation attaque launch
  (Variables|Default|SetDegatOverlaped true)
  (bind _angle (Timeline|Timeline_0 Play)
    (:Update
      (bind _res (CallFunction|EaseQuadOut _angle))
      (Transformation|SetRelativeRotation (Variables|Default|GetAnimCrino) (Math|Rotator|MakeRotator 0.0 0.0 (/ _res 5.0)) false false)
      (Variables|Default|SetDegatCrinoHere? true))))

(event Game|Damage|EventAnyDamage
  (params (Damage :type Float%20%28single-precision%29) (DamageType :type Damage%20Type%20Object%20Reference) (InstigatedBy :type Controller%20Object%20Reference) (DamageCauser :type Actor%20Object%20Reference))
  ;[1 0.9343 0 0.5] Gestion des dégâts sur le mannequin
  ;;[1 0.00746 0 0.5] Baisse la frustration quand le mannequin prend des dégâts
  (bind _asbp_third_person_character (Utilities|Casting|CastToBP_ThirdPersonCharacter (Game|GetPlayerCharacter 0)))
  (Variables|/Game/MyContent/BP_ThirdPersonCharacter.BP_ThirdPersonCharacter_C|SetFrustration _asbp_third_person_character (- (Variables|/Game/MyContent/BP_ThirdPersonCharacter.BP_ThirdPersonCharacter_C|GetFrustration _asbp_third_person_character) Damage))
  ;;[1 0.8187 0 0.5] L'ennemi perd de la vie quand il prend des dégâts, il passe en mode ragdoll lorsque ses PV sont à 0
  (Variables|Default|SetHPCRI (- (Variables|Default|GetHPCRI) Damage))
  (if (<= (Variables|Default|GetHPCRI) 0)
    (Development|PrintString "Hello")
    (Variables|Default|SetDED? true)))

(event EventBeginPlay
  ;[0.15 0.15 0.15 0.5] Verifie que le joueur est en mode frustré
  (Variables|Default|SetDegatCrinoHere? false)
  (Utilities|FlowControl|DelayUntilNextTick :!label _label)
  (bind _asbp_third_person_character (Utilities|Casting|CastToBP_ThirdPersonCharacter (Game|GetPlayerCharacter 0)))
  (if (Variables|/Game/MyContent/BP_ThirdPersonCharacter.BP_ThirdPersonCharacter_C|GetEnragé _asbp_third_person_character)
    ;[0.15 0.15 0.15 0.5] Fait une rotation avant de s'arreter, verifie si le joueur est toujours frustré avant de recommencer dans l'autre sens
    (Variables|Default|SetDegatCrinoHere? true)
    (Utilities|FlowControl|FlipFlop
      (:A
        (bind _angle (Timeline|Timeline Play)
          (:Update
            (bind _res (CallFunction|EaseQuadOut _angle))
            (Transformation|SetRelativeRotation (Variables|Default|GetAnimCrino) (Math|Rotator|MakeRotator 0.0 0.0 (/ _res 5.0)) false false))
          (:Finished
            (Variables|Default|SetDegatCrinoHere? false)
            (Utilities|FlowControl|Delay 5.0)
            (goto _label))))
      (:B
        (Timeline|Timeline Reverse)))
    (else
      (goto _label))))

(fn ConstructionScript)