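; BP_Computer1 is a puzzle computer that opens once two shelf placement objects are correct.
; Computer1Open checks the Shelf_Placement and Shelf_Placement_Child actors, swaps the mesh to an open laptop and sets Opening1.
; While open, overlapping its Box registers it as the character's Computer1Proche, which per comments drives interaction UI.
; End overlap compares the character to self rather than that reference, so its clearing branch never matches.
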(event OnComponentBeginOverlap(Box)
  (params (OverlappedComponent :type Primitive%20Component%20Object%20Reference) (OtherActor :type Actor%20Object%20Reference) (OtherComp :type Primitive%20Component%20Object%20Reference) (OtherBodyIndex :type Integer) (bFromSweep :type Boolean) (SweepResult :type Hit%20Result%20Structure%20%28by%20ref%29))
  ;[0.5765 0 1 0.502] Affiche l'UI d'interaction que lorsqu'il est est en phase 1, definit la possibilité de lancer l'event custon puzzle launch (cet event se lance selon l'affichage de l'UI)
  (bind _asbp_third_person_character (Utilities|Casting|CastToBP_ThirdPersonCharacter OtherActor))
  (if (Variables|Default|GetOpening1)
    (Variables|/Game/MyContent/BP_ThirdPersonCharacter.BP_ThirdPersonCharacter_C|SetComputer1Proche _asbp_third_person_character self)
    (else
      (Variables|/Game/MyContent/BP_ThirdPersonCharacter.BP_ThirdPersonCharacter_C|SetComputer1Proche _asbp_third_person_character 0))))

(event OnComponentEndOverlap(Box)
  (params (OverlappedComponent :type Primitive%20Component%20Object%20Reference) (OtherActor :type Actor%20Object%20Reference) (OtherComp :type Primitive%20Component%20Object%20Reference) (OtherBodyIndex :type Integer))
  ;[0.5765 0 1 0.502] Fait disparaitre l'UI
  (bind _asbp_third_person_character (Utilities|Casting|CastToBP_ThirdPersonCharacter OtherActor))
  (if (== _asbp_third_person_character self)
    (Variables|/Game/MyContent/BP_ThirdPersonCharacter.BP_ThirdPersonCharacter_C|SetComputer1Proche _asbp_third_person_character 0)))

(event Custom|Computer1Open
  ;[0 1 0.3529 0.502] Ne se déclenche qui les deux objets sont posés sur leurs emplacements spécifiques
  (bind _returnvalue (Actor|GetActorOfClass "/Game/MyContent/Enigme/PuzzlePlacement/Shelf_Placement.Shelf_Placement_C"))
  (bind _returnvalue_2 (Actor|GetActorOfClass "/Game/MyContent/Enigme/PuzzlePlacement/Shelf_Placement_Child.Shelf_Placement_Child_C"))
  (if (and (Variables|/Game/MyContent/Enigme/PuzzlePlacement/Shelf_Placement.Shelf_Placement_C|GetCorrect _returnvalue_2) (Variables|/Game/MyContent/Enigme/PuzzlePlacement/Shelf_Placement.Shelf_Placement_C|GetCorrect _returnvalue))
    (Components|StaticMesh|SetStaticMesh (Variables|Default|GetCube) "/Game/PROPS/PC_OPEN/LaptopOpen.LaptopOpen")
    (Variables|Default|SetOpening1 true)
    (Development|PrintString "Hello")))

(fn ConstructionScript)