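; BP_Computer2 is a puzzle-placement computer meant to open once two objects sit correctly and become interactable by the player, but its logic is currently disconnected.
; The overlap and Computer2Open events are empty.
; Orphaned nodes would check two actors' Correct flags, turn the cube blue, set Opening2, and assign or clear Computer2Proche on the third-person character.
; One branch clears ComputerProche instead of Computer2Proche.
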(event OnComponentBeginOverlap(Box)
  (params (OverlappedComponent :type Primitive%20Component%20Object%20Reference) (OtherActor :type Actor%20Object%20Reference) (OtherComp :type Primitive%20Component%20Object%20Reference) (OtherBodyIndex :type Integer) (bFromSweep :type Boolean) (SweepResult :type Hit%20Result%20Structure%20%28by%20ref%29))
  ;[0.5765 0 1 0.502] Affiche l'UI d'interaction que lorsqu'il est est en phase 1, definit la possibilité de lancer l'event custon puzzle launch (cet event se lance selon l'affichage de l'UI)
)

(event OnComponentEndOverlap(Box)
  (params (OverlappedComponent :type Primitive%20Component%20Object%20Reference) (OtherActor :type Actor%20Object%20Reference) (OtherComp :type Primitive%20Component%20Object%20Reference) (OtherBodyIndex :type Integer))
  ;[0.5765 0 1 0.502] Fait disparaitre l'UI
)

(event Custom|Computer2Open
  ;[0 1 0.3529 0.502] Ne se déclenche qui les deux objets sont posés sur leurs emplacements spécifiques
)

(fn ConstructionScript)