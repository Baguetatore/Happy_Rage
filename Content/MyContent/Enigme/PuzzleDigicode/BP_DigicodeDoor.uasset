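; BP_DigicodeDoor is a puzzle door that opens when the player has entered the correct digicode.
; Its Digicodeappear event confirms the player is BP_ThirdPersonCharacter, then branches on the Codecorrect flag.
; If true, a Timeline drives the Cube's relative yaw to swing it open.
; Otherwise it creates the UI_Digicode widget, shows the cursor and switches to Game and UI input focused on the keypad.
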(event Custom|Digicodeappear
  (bind _returnvalue (Game|GetPlayerController 0))
  ;[1 1 1] Animation ouvrir une porte qui si le joueur rentre le bon digicode
  (Utilities|Casting|CastToBP_ThirdPersonCharacter (Game|GetPlayerCharacter 0))
  (if (Variables|Default|GetCodecorrect?)
    (bind _angle (Timeline|Timeline Play)
      (:Update
        (Transformation|SetRelativeRotation (Variables|Default|GetCube) (Math|Rotator|MakeRotator 0.0 0.0 _angle) false false)))
    (else
      (bind _returnvalue_2 (UserInterface|CreateWidget "/Game/MyContent/Enigme/PuzzleDigicode/UI_Digicode.UI_Digicode_C"))
      (UserInterface|Viewport|AddtoViewport _returnvalue_2 0)
      (Variables|/Script/Engine.PlayerController|SetbShowMouseCursor _returnvalue true)
      (Input|SetInputModeGameandUI _returnvalue _returnvalue_2 "DoNotLock" true false))))

(fn ConstructionScript)