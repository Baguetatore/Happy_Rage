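; BP_Chevalet1 is a physical prop actor whose cube reacts to the state of the third-person player character.
; Every tick it enables custom depth on the cube while the player's ChevaletProche reference is valid, without checking that it points to this actor.
; Tick also switches off the cube's gravity while the player's IsZehef flag is true.
; Cube hits play a 2D collapse sound, and BarksCoffee calls a positional sound at the Box with no sound set.
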(event OnComponentHit(Cube)
  (params (HitComponent :type Primitive%20Component%20Object%20Reference) (OtherActor :type Actor%20Object%20Reference) (OtherComp :type Primitive%20Component%20Object%20Reference) (NormalImpulse :type Vector :default "0, 0, 0") (Hit :type Hit%20Result%20Structure%20%28by%20ref%29))
  (Audio|PlaySound2D "/Game/StarterContent/Audio/Collapse01.Collapse01" 1.0 1.0 0.0 0 0))

(event Custom|Barks%20Coffee
  (Audio|PlaySoundatLocation 0 (Transformation|GetWorldLocation (Variables|Default|GetBox)) "0, 0, 0" 1.0 1.0 0.0 0 0 0 0))

(event EventBeginPlay)

(event Collision|EventActorBeginOverlap
  (params (OtherActor :type Actor%20Object%20Reference)))

(event EventTick
  (params (DeltaSeconds :type Float%20%28single-precision%29))
  (bind _asbp_third_person_character (Utilities|Casting|CastToBP_ThirdPersonCharacter (Game|GetPlayerCharacter 0)))
  (Utilities|FlowControl|Sequence
    (:then_0
      (Utilities|IsValid (Variables|/Game/MyContent/BP_ThirdPersonCharacter.BP_ThirdPersonCharacter_C|GetChevaletProche _asbp_third_person_character)
        (:Is%20Valid
          (Rendering|SetRenderCustomDepth (Variables|Default|GetCube) true))
        (:Is%20Not%20Valid
          (Rendering|SetRenderCustomDepth (Variables|Default|GetCube) false))))
    (:then_1
      (if (Variables|/Game/MyContent/BP_ThirdPersonCharacter.BP_ThirdPersonCharacter_C|GetIsZehef _asbp_third_person_character)
        (Physics|SetEnableGravity (Variables|Default|GetCube) false)
        (else
          (Physics|SetEnableGravity (Variables|Default|GetCube) true))))))

(fn ConstructionScript)