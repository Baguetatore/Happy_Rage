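; BP_Sac_à_dos is a backpack actor whose LaptopClosed component reacts to the player's enraged state.
; Every Tick it casts the player character to BP_ThirdPersonCharacter and disables the component's gravity while Enragé is true, restoring it otherwise.
; It also overrides the component's mass each Tick through a hard-coded true branch, so the heavier alternative never runs.
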(event EventBeginPlay)

(event Collision|EventActorBeginOverlap
  (params (OtherActor :type Actor%20Object%20Reference)))

(event EventTick
  (params (DeltaSeconds :type Float%20%28single-precision%29))
  (bind _asbp_third_person_character (Utilities|Casting|CastToBP_ThirdPersonCharacter (Game|GetPlayerCharacter 0)))
  (Utilities|FlowControl|Sequence
    (:then_1
      (if (Variables|/Game/MyContent/BP_ThirdPersonCharacter.BP_ThirdPersonCharacter_C|GetEnragé _asbp_third_person_character)
        (Physics|SetEnableGravity (Variables|Default|GetLaptopClosed) false)
        (else
          (Physics|SetEnableGravity (Variables|Default|GetLaptopClosed) true))))
    (:then_2
      (if true
        (Class|PrimitiveComponent|SetMassOverrideinKg (Variables|Default|GetLaptopClosed) "None" 1e+02 true)
        (else
          (Class|PrimitiveComponent|SetMassOverrideinKg (Variables|Default|GetLaptopClosed) "None" 5e+02 true))))))

(fn ConstructionScript)