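; BP_PCOuvert4 is an actor with a Cube mesh that highlights through custom depth and can play a bark sound.
; Every tick it casts the player to BP_ThirdPersonCharacter and enables the Cube's custom depth while that character's PCO4Proche reference is valid.
; The Barks event plays a sound at the Cube's world location; nothing in this graph calls it.
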(event Custom|Barks
  (Audio|PlaySoundatLocation 0 (Transformation|GetWorldLocation (Variables|Default|GetCube)) "0, 0, 0" 1.0 1.0 0.0 0 0 0 0))

(event EventBeginPlay)

(event Collision|EventActorBeginOverlap
  (params (OtherActor :type Actor%20Object%20Reference)))

(event EventTick
  (params (DeltaSeconds :type Float%20%28single-precision%29))
  (bind _asbp_third_person_character (Utilities|Casting|CastToBP_ThirdPersonCharacter (Game|GetPlayerCharacter 0)))
  (Utilities|IsValid (Variables|/Game/MyContent/BP_ThirdPersonCharacter.BP_ThirdPersonCharacter_C|GetPCO4Proche _asbp_third_person_character)
    (:Is%20Valid
      (Rendering|SetRenderCustomDepth (Variables|Default|GetCube) true))
    (:Is%20Not%20Valid
      (Rendering|SetRenderCustomDepth (Variables|Default|GetCube) false))))

(fn ConstructionScript)